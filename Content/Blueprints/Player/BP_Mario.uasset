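; Player character for a Mario-style side-scroller, with Enhanced Input movement, jumping and fireballs.
; Tick eases the camera forward only along X, spawning a blocking border when the player reaches the left screen edge, re-armed as the camera advances.
; PlayerLevel tracks power-ups: timelines drive scale and mesh swaps, and the top tier allows two live fireballs.
; Injuries downgrade with a one-second cooldown or trigger an animated death that loads MainUI.
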(event `self.ReceiveBeginPlay`
  ;[1 1 1] 启用自己的输入映射情景
  (bind _asbp_my_player_controller (cast `/Game/Blueprints/Gameplay/BP_MyPlayerController` (`self.GetController`)))
  (set `self.Player Controller Ref` _asbp_my_player_controller)
  (bind _returnvalue (pcsubsystem `EnhancedInputLocalPlayerSubsystem` _asbp_my_player_controller))
  (`/Engine/EditorBlueprintResources/StandardMacros.IsValid` _returnvalue
    (:`Is Valid`
      (`EnhancedInputSubsystemInterface.AddMappingContext` _returnvalue "/Game/Blueprints/Player/Input/IMC_Operate.IMC_Operate" 0 (struct))
      ;[1 1 1] 设置摄像机初始位置，并且启用tick事件
      (`SceneComponent.K2_SetWorldLocation` (`self.CameraBoom`) (500.0 0.0 400.0) false false)
      (`KismetSystemLibrary.Delay` 0.1)
      (`self.SetActorTickEnabled` true))))

(event `EnhancedInput|/Game/Blueprints/Player/Input/InputActions/IA_Move`
  (params (ActionValue :type "Float (double-precision)") (ElapsedSeconds :type "Float (double-precision)") (TriggeredSeconds :type "Float (double-precision)") (InputAction :type "InputAction Object Reference" :default "/Game/Blueprints/Player/Input/InputActions/IA_Move.IA_Move"))
  ;[1 1 1] 左右移动
  (:`Triggered`
    (`self.AddMovementInput` (1.0 0.0 0.0) ActionValue)))

(event `EnhancedInput|/Game/Blueprints/Player/Input/InputActions/IA_Jump`
  (params (ActionValue :type Boolean) (ElapsedSeconds :type "Float (double-precision)") (TriggeredSeconds :type "Float (double-precision)") (InputAction :type "InputAction Object Reference" :default "/Game/Blueprints/Player/Input/InputActions/IA_Jump.IA_Jump"))
  ;[1 1 1] 跳跃
  (:`Started`
    (`self.Jump`))
  (:`Completed`
    (`self.StopJumping`)))

(event `self.ReceiveTick`
  (params (DeltaSeconds :type "Float (single-precision)"))
  (bind (_returnvalue_x _returnvalue_y _returnvalue_z) (`KismetMathLibrary.BreakVector` (`self.K2_GetActorLocation`)))
  (bind _returnvalue_x_2 (`KismetMathLibrary.BreakVector` (`KismetMathLibrary.VInterpTo` (`SceneComponent.K2_GetComponentLocation` (`self.CameraBoom`)) (+ (`self.K2_GetActorLocation`) (500.0 0.0 0.0)) (`GameplayStatics.GetWorldDeltaSeconds`) 2.0)))
  (`|ExecutionSequence`
    (:`then_0`
      ;[1 1 1] 摄像机缓动与停止
      (if (>= _returnvalue_x_2 (`self.InitialCameraLocation`))
        (set `self.InitialCameraLocation` _returnvalue_x_2)
        (`SceneComponent.K2_SetWorldLocation` (`self.CameraBoom`) (`KismetMathLibrary.MakeVector` _returnvalue_x_2 0.0 400.0) false false)
        (goto _label :!via `Reset`)))
    (:`then_1`
      ;[1 1 1] 角色超过屏幕边界生成阻挡边界
      (if (not (>= (`KismetMathLibrary.BreakVector2D` (`PlayerController.ProjectWorldLocationToScreen` (`self.Player Controller Ref`) (`self.K2_GetActorLocation`) false)) 18.0))
        (`/Engine/EditorBlueprintResources/StandardMacros.DoOnce` false :!label _label
          (:`Completed`
            (`|SpawnActorFromClass` "/Game/Blueprints/Actors/Environment/ABP_Border.ABP_Border_C" (`KismetMathLibrary.MakeTransform` (`KismetMathLibrary.MakeVector` (- _returnvalue_x 50.0) _returnvalue_y _returnvalue_z)) "Undefined" "MultiplyWithRoot" null null)))))))

(event `PlayerAddScale`
  ;[1 1 1] 角色的放大和缩小
  (`GameplayStatics.SetGlobalTimeDilation` 0.2)
  (`GameplayStatics.PlaySound2D` "/Game/Assets/Audio/Mario_Powerup.Mario_Powerup" 1.0 1.0 0.0 null null)
  (set `self.PlayerLevel` 1)
  (`/Game/Blueprints/Gameplay/BP_MyPlayerController.Add Score` (`/Game/Blueprints/FunctionLibrary/BP_MyFunctionLibrary.GetMyPlayerController`) 1000)
  (bind (_direction _scale) (`Timeline|TL_PlayerScale` :!via `PlayFromStart` :!label _label_2)
    (:`Update`
      (`self.SetActorScale3D` (* _scale (1.0 1.0 1.0))))
    (:`Finished`
      (`GameplayStatics.SetGlobalTimeDilation` 1.0))))

(event `PlayerReduceScale`
  ;[1 1 1] 角色的放大和缩小
  (`GameplayStatics.PlaySound2D` "/Game/Assets/Audio/Mario_Warp.Mario_Warp" 1.0 1.0 0.0 null null)
  (set `self.PlayerLevel` 0)
  (goto _label_2 :!via `ReverseFromEnd`))

(event `PlayerColorChange`
  ;[1 1 1] 改变角色颜色
  (bind (_direction _meshindex) (`Timeline|时间轴` :!via `PlayFromStart` :!label _label_3)
    (:`Update`
      (set `SkeletalMeshComponent.SkeletalMeshAsset` (select `int` (`KismetMathLibrary.FTrunc` _meshindex) :`0` "/Game/Assets/FallTower/Assets/Character/SK_Character_8.SK_Character_8" :`1` "/Game/Assets/FallTower/Assets/Character/SK_Character_2.SK_Character_2" :`2` "/Game/Assets/FallTower/Assets/Character/SK_Character_3.SK_Character_3" :`3` "/Game/Assets/FallTower/Assets/Character/SK_Character_4.SK_Character_4" :`4` "/Game/Assets/FallTower/Assets/Character/SK_Character_5.SK_Character_5" :`5` "/Game/Assets/FallTower/Assets/Character/SK_Character_6.SK_Character_6" :`6` "/Game/Assets/FallTower/Assets/Character/SK_Character.SK_Character" :`7` "/Game/Assets/FallTower/Assets/Character/SK_Character_7.SK_Character_7" :!type "SkeletalMesh Object Reference") (`self.Mesh`)))
    (:`Finished`
      (`/Engine/EditorBlueprintResources/StandardMacros.IncrementInt` (`self.PlayerLevel`)))))

(event `PlayerColorDefault`
  ;[1 1 1] 改变角色颜色
  (goto _label_3 :!via `ReverseFromEnd`))

(event `EnhancedInput|/Game/Blueprints/Player/Input/InputActions/IA_Attack`
  (params (ActionValue :type Boolean) (ElapsedSeconds :type "Float (double-precision)") (TriggeredSeconds :type "Float (double-precision)") (InputAction :type "InputAction Object Reference" :default "/Game/Blueprints/Player/Input/InputActions/IA_Attack.IA_Attack"))
  ;[1 1 1] 角色发射子弹
  (:`Started`
    (if (== (`self.PlayerLevel`) 2)
      (bind _outactors (`GameplayStatics.GetAllActorsOfClass` "/Game/Blueprints/Actors/Ammo/ABP_Ammo.ABP_Ammo_C"))
      (bind _output_get (set `self.AmmoArray` _outactors))
      (bind _output_get_2 (set `self.AmmoNumber` (`KismetArrayLibrary.Array_Length` _output_get)))
      (if (< _output_get_2 2)
        (`|SpawnActorFromClass` "/Game/Blueprints/Actors/Ammo/ABP_Ammo.ABP_Ammo_C" (`SceneComponent.K2_GetComponentToWorld` (`self.Arrow1`)) "Undefined" "MultiplyWithRoot" null null)
        (`GameplayStatics.PlaySoundAtLocation` "/Game/Assets/Audio/Mario_Fireball.Mario_Fireball" (`self.K2_GetActorLocation`) (struct) 1.0 1.0 0.0 null null null null)))))

(event `PlayerInjured`
  ;[1 1 1] 角色的受伤逻辑
  (`/Engine/EditorBlueprintResources/StandardMacros.DoOnce` false :!label _label_4
    (:`Completed`
      (switch `int` (`self.PlayerLevel`)
        (:`0`
          (`self.PlayerDies`))
        (:`1`
          (`self.PlayerReduceScale`)
          (`KismetSystemLibrary.Delay` 1.0 :!label _label_5)
          (goto _label_4 :!via `Reset`))
        (:`2`
          (`|ExecutionSequence`
            (:`then_0`
              (`self.PlayerReduceScale`))
            (:`then_1`
              (`self.PlayerColorDefault`))
            (:`then_2`
              (goto _label_5))))))))

(event `PlayerDies`
  (bind (_playerdeathlocation_x _playerdeathlocation_y _playerdeathlocation_z) (`KismetMathLibrary.BreakVector` (`self.PlayerDeathLocation`)))
  ;[1 1 1] 角色的死亡逻辑
  (`/Engine/EditorBlueprintResources/StandardMacros.DoOnce` false
    (:`Completed`
      (`self.PlayerDeath`)
      (set `self.PlayerDeathLocation` (`self.K2_GetActorLocation`))
      ;;[1 1 1] 死亡动画以及音效
      (`GameplayStatics.PlaySound2D` "/Game/Assets/Audio/Mario_Die.Mario_Die" 1.0 1.0 0.0 null null)
      (`self.DisableInput` self (`/Game/Blueprints/FunctionLibrary/BP_MyFunctionLibrary.GetMyPlayerController`))
      (`GameplayStatics.SpawnEmitterAtLocation` "/Game/StarterContent/Particles/P_Explosion.P_Explosion" (`self.K2_GetActorLocation`))
      (`ActorComponent.Deactivate` (`self.CharacterMovement`))
      (`PrimitiveComponent.SetCollisionEnabled` (`self.CapsuleComponent`) "NoCollision")
      (`SkeletalMeshComponent.PlayAnimation` (`self.Mesh`) "/Game/Assets/FallTower/Assets/Character/Animations/AS_Jump_Fall.AS_Jump_Fall" false)
      (`SceneComponent.K2_DetachFromComponent` (`self.Mesh`) "KeepWorld" "KeepWorld" "KeepWorld" true)
      (bind (_direction _movement) (`Timeline|TL_PlayerDeath` :!via `PlayFromStart`)
        (:`Update`
          (`SceneComponent.K2_SetRelativeLocationAndRotation` :`self` (`self.Mesh`) :`NewLocation` (`KismetMathLibrary.MakeVector` _playerdeathlocation_x _playerdeathlocation_y (+ _movement _playerdeathlocation_z)))
          (`KismetSystemLibrary.Delay` 3.0)
          (`self.K2_DestroyActor`)
          (`GameplayStatics.OpenLevel` "MainUI"))))))

(fn `UserConstructionScript`)