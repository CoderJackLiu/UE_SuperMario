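; Power-up mushroom that moves on its own and grows Mario when he touches it.
; Tick feeds a stored X direction into movement input, and a FlipFlop switches it between -1 and 1 on capsule hits with actors not tagged Plane.
; A Player-tagged BP_Mario overlap triggers PlayerAddScale once, spawns a floating score at the mushroom's location, then destroys it.
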(event `self.ReceiveBeginPlay`)

(event `self.ReceiveTick`
  (params (DeltaSeconds :type "Float (single-precision)"))
  (`self.AddMovementInput` (`KismetMathLibrary.MakeVector` (`self.World Direction X`))))

(event `self.CapsuleComponent.OnComponentHit`
  (params (HitComponent :type "PrimitiveComponent Object Reference") (OtherActor :type "Actor Object Reference") (OtherComp :type "PrimitiveComponent Object Reference") (NormalImpulse :type "Vector Structure") (Hit :type "HitResult Structure (by ref)"))
  (if (not (`self.ActorHasTag` OtherActor "Plane"))
    (`/Engine/EditorBlueprintResources/StandardMacros.FlipFlop`
      (:`A`
        (set `self.World Direction X` -1.0))
      (:`B`
        (set `self.World Direction X` 1.0)))))

(event `self.CapsuleComponent.OnComponentBeginOverlap`
  (params (OverlappedComponent :type "PrimitiveComponent Object Reference") (OtherActor :type "Actor Object Reference") (OtherComp :type "PrimitiveComponent Object Reference") (OtherBodyIndex :type Integer) (bFromSweep :type Boolean) (SweepResult :type "HitResult Structure (by ref)"))
  (if (`self.ActorHasTag` OtherActor "Player")
    (bind _asbp_mario (cast `/Game/Blueprints/Player/BP_Mario` OtherActor))
    (`/Engine/EditorBlueprintResources/StandardMacros.DoOnce` false
      (:`Completed`
        (`/Game/Blueprints/Player/BP_Mario.PlayerAddScale` _asbp_mario)
        (`|SpawnActorFromClass` "/Game/Blueprints/Actors/UI/ABP_FloatUI.ABP_FloatUI_C" (`KismetMathLibrary.MakeTransform` (`self.K2_GetActorLocation`)) "Undefined" "MultiplyWithRoot" null 1000 null)
        (`self.K2_DestroyActor`)))))

(fn `UserConstructionScript`)