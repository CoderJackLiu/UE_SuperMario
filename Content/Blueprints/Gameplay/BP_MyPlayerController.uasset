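; Player controller that owns the game HUD and tracks coins, score and lives in what appears to be a Mario-style game.
; BeginPlay creates and shows the WB_GameMain widget, then switches to game-only input with the cursor hidden.
; AddCoinsNumber feeds points into AddScore, rolls every hundred coins into an extra life with a 1-up sound, and both events cache zero-padded text versions of their totals.
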(event `self.ReceiveBeginPlay`
  (bind _returnvalue (`|CreateWidget` "/Game/Blueprints/UI/WB_GameMain.WB_GameMain_C"))
  (set `self.WB_GameMainRef` _returnvalue)
  (`UserWidget.AddToViewport` _returnvalue 0)
  (`WidgetBlueprintLibrary.SetInputMode_GameOnly` self)
  (set `self.bShowMouseCursor` false))

(event `self.ReceiveTick`
  (params (DeltaSeconds :type "Float (single-precision)")))

(event `Add Coins Number`
  (params (PickupCoins :type Integer))
  (bind _returnvalue (+ PickupCoins (`self.CoinsNumber`)))
  ;[1 1 1] 添加金币数量
  (`self.Add Score` (* PickupCoins 200))
  (if (>= _returnvalue 100)
    (set `self.CoinsNumber` (`KismetMathLibrary.Clamp` (- _returnvalue 100) 0 99))
    (`/Engine/EditorBlueprintResources/StandardMacros.IncrementInt` (`self.Lives`)
      (:`  `
        (`GameplayStatics.PlaySound2D` "/Game/Assets/Audio/Mario_1up.Mario_1up" 1.0 1.0 0.0 null null)))
    (else
      (set `self.CoinsNumber` (`KismetMathLibrary.Clamp` _returnvalue 0 99))))
  (set `self.Coins` (`KismetTextLibrary.Conv_IntToText` (`self.CoinsNumber`) false false 2 2)))

(event `Add Score`
  (params (`Score To Add` :type Integer))
  ;[1 1 1] 添加分数
  (bind _output_get (set `self.ScoreNumber` (+ `Score To Add` (`self.ScoreNumber`))))
  (set `self.Score` (`KismetTextLibrary.Conv_IntToText` _output_get false false 6 6)))

(fn `UserConstructionScript`)