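; Mushroom enemy for a Mario-style game that walks along the X axis once the player enters its Sphere1 trigger.
; Capsule hits on anything not tagged Plane flip-flop its direction, and Sphere overlaps injure the player.
; A player hit on the Box, filtered by downward impact normal, squashes it and destroys it after a delay.
; Ammo hits destroy it immediately with effects; both kills award score with floating text.
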(event `self.ReceiveTick`
  (params (DeltaSeconds :type "Float (single-precision)"))
  (if (`self.Move?`)
    (`self.AddMovementInput` (`KismetMathLibrary.MakeVector` (`KismetMathLibrary.SelectFloat` 1.0 -1.0 (`self.MoveRight?`))))))

(event `self.CapsuleComponent.OnComponentHit`
  (params (HitComponent :type "PrimitiveComponent Object Reference") (OtherActor :type "Actor Object Reference") (OtherComp :type "PrimitiveComponent Object Reference") (NormalImpulse :type "Vector Structure") (Hit :type "HitResult Structure (by ref)"))
  (if (not (`self.ActorHasTag` OtherActor "Plane"))
    (`/Engine/EditorBlueprintResources/StandardMacros.FlipFlop`
      (:`A`
        (set `self.MoveRight?` true))
      (:`B`
        (set `self.MoveRight?` false)))))

(event `self.Sphere.OnComponentBeginOverlap`
  (params (OverlappedComponent :type "PrimitiveComponent Object Reference") (OtherActor :type "Actor Object Reference") (OtherComp :type "PrimitiveComponent Object Reference") (OtherBodyIndex :type Integer) (bFromSweep :type Boolean) (SweepResult :type "HitResult Structure (by ref)"))
  ;[1 1 1] 重叠攻击玩家的逻辑
  (if (`self.ActorHasTag` OtherActor "Player")
    (bind _asbp_mario (cast `/Game/Blueprints/Player/BP_Mario` OtherActor))
    (`/Game/Blueprints/Player/BP_Mario.PlayerInjured` _asbp_mario)))

(event `self.Box.OnComponentHit`
  (params (HitComponent :type "PrimitiveComponent Object Reference") (OtherActor :type "Actor Object Reference") (OtherComp :type "PrimitiveComponent Object Reference") (NormalImpulse :type "Vector Structure") (Hit :type "HitResult Structure (by ref)"))
  ;[1 1 1] 踩踏逻辑
  (if (and (`self.ActorHasTag` OtherActor "Player") (== (`.ImpactNormal` (`GameplayStatics.BreakHitResult` Hit)) (0.0 0.0 -1.0) :`ErrorTolerance` 0.1))
    (`|ExecutionSequence`
      (:`then_0`
        ;;[1 1 1] 播放音效和特效
        (`GameplayStatics.PlaySound2D` "/Game/Assets/Audio/Mario_Squish.Mario_Squish" 1.0 1.0 0.0 null null)
        (`PrimitiveComponent.SetCollisionEnabled` (`self.Box`) "NoCollision")
        (`PrimitiveComponent.SetCollisionEnabled` (`self.Sphere`) "NoCollision")
        (`ActorComponent.K2_DestroyComponent` (`self.Box`))
        (`SceneComponent.SetWorldScale3D` (`self.CapsuleComponent`) (1.0 1.0 0.3)))
      (:`then_1`
        ;;[1 1 1] 禁止移动
        (`CharacterMovementComponent.DisableMovement` (`self.CharacterMovement`)))
      (:`then_2`
        ;;[1 1 1] 添加积分
        (`|SpawnActorFromClass` "/Game/Blueprints/Actors/UI/ABP_FloatUI.ABP_FloatUI_C" (`KismetMathLibrary.MakeTransform` (`self.K2_GetActorLocation`)) "Undefined" "MultiplyWithRoot" null 100 null)
        (`/Game/Blueprints/Gameplay/BP_MyPlayerController.Add Score` (`/Game/Blueprints/FunctionLibrary/BP_MyFunctionLibrary.GetMyPlayerController`) 100))
      (:`then_3`
        ;;[1 1 1] 销毁
        (`KismetSystemLibrary.Delay` 0.5)
        (`self.K2_DestroyActor`)))))

(event `self.Sphere.OnComponentHit`
  (params (HitComponent :type "PrimitiveComponent Object Reference") (OtherActor :type "Actor Object Reference") (OtherComp :type "PrimitiveComponent Object Reference") (NormalImpulse :type "Vector Structure") (Hit :type "HitResult Structure (by ref)"))
  ;[1 1 1] 蘑菇怪被子弹击中逻辑
  (if (`self.ActorHasTag` OtherActor "Ammo")
    (bind _asabp_ammo (cast `/Game/Blueprints/Actors/Ammo/ABP_Ammo` OtherActor))
    (`self.K2_DestroyActor` _asabp_ammo)
    (`|ExecutionSequence`
      (:`then_0`
        (`|SpawnActorFromClass` "/Game/Blueprints/Actors/UI/ABP_FloatUI.ABP_FloatUI_C" (`KismetMathLibrary.MakeTransform` (`self.K2_GetActorLocation`)) "Undefined" "MultiplyWithRoot" null 100 null)
        (`/Game/Blueprints/Gameplay/BP_MyPlayerController.Add Score` (`/Game/Blueprints/FunctionLibrary/BP_MyFunctionLibrary.GetMyPlayerController`) 100))
      (:`then_1`
        (`/Game/Blueprints/FunctionLibrary/BP_MyFunctionLibrary.PlaySoundAndVFX` "/Game/Assets/Audio/Mario_Kick.Mario_Kick" null (0.0 0.0 0.0) "/Game/InfinityBladeEffects/Effects/FX_Monsters/FX_Monster_Gruntling/FlameThrower/P_FlameExplode.P_FlameExplode" (`SceneComponent.K2_GetComponentLocation` (`self.Sphere`)))
        (`self.K2_DestroyActor`)))))

(event `self.Sphere1.OnComponentBeginOverlap`
  (params (OverlappedComponent :type "PrimitiveComponent Object Reference") (OtherActor :type "Actor Object Reference") (OtherComp :type "PrimitiveComponent Object Reference") (OtherBodyIndex :type Integer) (bFromSweep :type Boolean) (SweepResult :type "HitResult Structure (by ref)"))
  (if (`self.ActorHasTag` OtherActor "Player")
    (`/Engine/EditorBlueprintResources/StandardMacros.DoOnce` false
      (:`Completed`
        (set `self.Move?` true)))))

(fn `UserConstructionScript`)