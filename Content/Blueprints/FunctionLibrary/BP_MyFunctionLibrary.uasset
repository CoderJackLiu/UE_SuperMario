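; Blueprint function library of shared helpers for a Mario game.
; PlaySoundAndVFX plays a 2D sound and spawns a Niagara system and a Cascade emitter, each at its own location, in one call.
; GetMyCharacter and GetMyPlayerController return player 0's pawn and controller, already cast to BP_Mario and BP_MyPlayerController.
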(fn `GetMyCharacter`
  (returns (`Character Ref` :type "/Game/Blueprints/Player/BP_Mario Object Reference"))
  (bind _asbp_mario (cast `/Game/Blueprints/Player/BP_Mario` (`GameplayStatics.GetPlayerCharacter` null)))
  (return _asbp_mario))

(fn `GetMyPlayerController`
  (returns (`Player Controller Ref` :type "/Game/Blueprints/Gameplay/BP_MyPlayerController Object Reference"))
  (bind _asbp_my_player_controller (cast `/Game/Blueprints/Gameplay/BP_MyPlayerController` (`GameplayStatics.GetPlayerController` null)))
  (return _asbp_my_player_controller))

(fn `PlaySoundAndVFX`
  (params (Sound :type "SoundBase Object Reference") (Niagara :type "NiagaraSystem Object Reference") (N_Location :type "Vector Structure") (Particle :type "ParticleSystem Object Reference") (P_Location :type "Vector Structure"))
  (`GameplayStatics.PlaySound2D` null Sound 1.0 1.0 0.0 null null)
  (`NiagaraFunctionLibrary.SpawnSystemAtLocation` null Niagara N_Location)
  (`GameplayStatics.SpawnEmitterAtLocation` null Particle P_Location))